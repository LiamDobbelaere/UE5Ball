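; BallCamera is a mouse-orbit follow camera that trails a FocusedPawn, presumably the ball.
; Mouse2D input accumulates into LookVector as yaw and pitch, with pitch clamped.
; Each Tick eases the actor to a point behind the pawn at fixed height, then turns it toward a point ahead along the look direction.
; Pitch therefore moves the aim point and shortens horizontal distance, while smoothing uses delta-time-scaled lerps.
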(event `InputVectorAxis|Mouse2D`
  (params (AxisValue :type "Vector Structure"))
  ;[1 1 1] Mouse orbit
  (bind _output_get (set `self.LookVector` (`KismetMathLibrary.MakeVector` (.x (+ AxisValue (`self.LookVector`))) (`KismetMathLibrary.ClampAngle` (.y (+ AxisValue (`self.LookVector`))) -45.0 45.0)))))

(event `self.ReceiveTick`
  (params (DeltaSeconds :type "Float (single-precision)"))
  (bind _returnvalue (* DeltaSeconds 10.0))
  (bind _returnvalue_2 (`self.K2_GetActorLocation` (`self.FocusedPawn`)))
  (bind _returnvalue_3 (`KismetMathLibrary.Normal` (`KismetMathLibrary.GetForwardVector` (`KismetMathLibrary.MakeRotator` 0.0 (.y (stale `InputVectorAxis|Mouse2D` _output_get)) (.x (stale `InputVectorAxis|Mouse2D` _output_get))))))
  (`self.K2_SetActorLocation` (`KismetMathLibrary.VLerp` (`self.K2_GetActorLocation`) (+ _returnvalue_2 (0.0 0.0 0.0) (`KismetMathLibrary.MakeVector` (.x (* _returnvalue_3 (`KismetMathLibrary.Conv_DoubleToVector` -200.0))) (.y (* _returnvalue_3 (`KismetMathLibrary.Conv_DoubleToVector` -200.0))) 50.0)) _returnvalue))
  (`self.K2_SetActorRotation` (`KismetMathLibrary.RLerp` (`self.K2_GetActorRotation`) (`KismetMathLibrary.FindLookAtRotation` (`self.K2_GetActorLocation`) (+ (* _returnvalue_3 (`KismetMathLibrary.Conv_DoubleToVector` 100.0)) _returnvalue_2)) _returnvalue true)))

(fn `UserConstructionScript`)