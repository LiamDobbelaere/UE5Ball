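; BallPawn is a pawn that rolls a physics sphere from player input and gets dirtier on hard impacts.
; Vertical and Horizontal axes share one impulse, built from camera-relative forward and right vectors and scaled by sphere mass and Speed.
; Hits above an impulse threshold increment Dirtiness, which drives a scalar parameter on the sphere's materials.
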(event `InputAxis|Vertical`
  (params (AxisValue :type "Float (single-precision)"))
  (bind _returnvalue (`self.K2_GetActorRotation` (`GameplayStatics.GetPlayerCameraManager` 0)))
  ;[1 1 1] Movement
  (`PrimitiveComponent.AddImpulse` (`self.Sphere`) (* (+ (* (`KismetMathLibrary.GetForwardVector` _returnvalue) AxisValue) (* (`KismetMathLibrary.GetRightVector` _returnvalue) (stale `InputAxis|Horizontal` AxisValue))) (* (`PrimitiveComponent.GetMass` (`self.Sphere`)) (`self.Speed`))) "None" false :!label _label))

(event `InputAxis|Horizontal`
  (params (AxisValue :type "Float (single-precision)"))
  ;[1 1 1] Movement
  (goto _label))

(event `self.ReceiveHit`
  (params (MyComp :type "PrimitiveComponent Object Reference") (Other :type "Actor Object Reference") (OtherComp :type "PrimitiveComponent Object Reference") (bSelfMoved :type Boolean) (HitLocation :type "Vector Structure") (HitNormal :type "Vector Structure") (NormalImpulse :type "Vector Structure") (Hit :type "HitResult Structure (by ref)"))
  (if (> (`KismetMathLibrary.VSize` NormalImpulse) 400.0)
    (bind _output_get (set `self.Dirtiness` (+ (`self.Dirtiness`) 0.01)))
    (`MeshComponent.SetScalarParameterValueOnMaterials` (`self.Sphere`) "Dirtiness" _output_get)))

(fn `UserConstructionScript`)